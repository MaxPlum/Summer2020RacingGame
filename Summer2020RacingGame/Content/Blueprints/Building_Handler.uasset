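; Building handler actor that procedurally assembles a modular, one-to-four-sided building from Building_Unit actors in its construction script.
; Width, height, depth and side count set the unit total; units are spawned or destroyed to match.
; One-shot bools trigger realignment, which chains walls around 90-degree corners, roofs the top floor and moves the handler above the building, or randomization of each unit's awning, rails and vent.
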(event Custom|Spawn%20Building%20Units
  (bind _building (Variables|Default|GetBuilding))
  (bind _height (Variables|Default|GetHeight))
  (bind _building_2 (Variables|Default|GetBuilding))
  (bind _building_3 (Variables|Default|GetBuilding))
  (bind _sides (Variables|Default|GetSides))
  (bind _width (Variables|Default|GetWidth))
  (bind _height_2 (Variables|Default|GetHeight))
  (bind _building_4 (Variables|Default|GetBuilding))
  (bind _depth (Variables|Default|GetDepth))
  (bind _sides_2 (Variables|Default|GetSides))
  (bind _building_5 (Variables|Default|GetBuilding))
  (bind _returnvalue (Utilities|Array|Length _building_2))
  (bind _returnvalue_2 (Utilities|Array|Length _building))
  (bind _returnvalue_3 (Utilities|Array|Length _building_3))
  (bind _returnvalue_4 (/ _sides 3))
  (bind _returnvalue_5 (/ _sides_2 2))
  (bind _returnvalue_6 (* _width _height_2))
  (bind _returnvalue_7 (* _height_2 _depth))
  (bind _returnvalue_8 (- _returnvalue_2 1))
  (bind _returnvalue_9 (- _returnvalue 1))
  (bind _returnvalue_10 (* _returnvalue_7 _returnvalue_5))
  (bind _returnvalue_11 (+ _returnvalue_4 1))
  (bind _returnvalue_12 (* _returnvalue_11 _returnvalue_6))
  (bind _output (Utilities|Array|Get(acopy) _building_4 _returnvalue_9))
  (bind _returnvalue_13 (+ _returnvalue_12 _returnvalue_10))
  (bind _building_mesh (Variables|/Game/Blueprints/Building_Unit.Building_Unit_C|GetBuilding%20Mesh _output))
  (bind _returnvalue_14 (- _returnvalue_13 _returnvalue_3))
  (bind _returnvalue_15 (Transformation|GetWorldTransform _building_mesh))
  (Math|Integer|CompareInt _returnvalue_14
    (:>
      ;[1 1 1] Add Necessary Number Of Building Units
      (Variables|Default|SetLoop%20Check true)
      (while (Variables|Default|GetLoop%20Check)
        ;;[1 1 1] Check If Unit Array Is Empty
        (if (== _returnvalue 0)
          (bind _returnvalue_16 (Game|SpawnActorfromClass "/Game/Blueprints/Building_Unit.Building_Unit_C" (Transformation|GetWorldTransform (Variables|Default|GetDefaultSceneRoot)) "AlwaysSpawn" 0 0))
          (Utilities|IsValid _returnvalue_16
            (:Is%20Valid
              (Utilities|Array|Add _building_5 _returnvalue_16)
              (Variables|Default|SetLoop%20Check (!= (+ (* (+ (/ (Variables|Default|GetSides) 3) 1) (* (Variables|Default|GetWidth) _height)) (* (* _height (Variables|Default|GetDepth)) (/ (Variables|Default|GetSides) 2))) (Utilities|Array|Length (Variables|Default|GetBuilding))) :!label _label))
            (:Is%20Not%20Valid
              (Variables|Default|SetLoop%20Check false :!label _label_2)))
          (else
            (bind _returnvalue_17 (Game|SpawnActorfromClass "/Game/Blueprints/Building_Unit.Building_Unit_C" (Math|Transform|MakeTransform (Math|Vector|MakeVector (+ (.x (.location _returnvalue_15)) 1.2e+03) (.y (.location _returnvalue_15)) (.z (.location _returnvalue_15))) (.rotation _returnvalue_15) (.scale _returnvalue_15)) "AlwaysSpawn" 0 0))
            (Utilities|IsValid _returnvalue_17
              (:Is%20Valid
                (Utilities|Array|Add _building_5 _returnvalue_17)
                (goto _label))
              (:Is%20Not%20Valid
                (goto _label_2)))))))
    (:<
      ;[1 1 1] Remove Excess Building Units
      (while (!= _returnvalue_14 0)
        (if (not (== _returnvalue_2 0))
          (Actor|DestroyActor (Utilities|Array|Get(acopy) _building _returnvalue_8))
          (Utilities|Array|RemoveIndex _building _returnvalue_8))))))

(fn ConstructionScript
  (CallFunction|SetBuildingDimensions)
  (CallFunction|SpawnBuildingUnits)
  (if (Variables|Default|GetRealign%20Building%20Units)
    (CallFunction|HandleBuildingRepositioning)
    (Variables|Default|SetRealign%20Building%20Units false))
  (if (Variables|Default|GetRandomize%20Building%20Details)
    (CallFunction|RandomizeBuildingUnitDetails)
    (Variables|Default|SetRandomize%20Building%20Details false)))

(fn SetBuildingDimensions
  (switch Utilities|FlowControl|Switch|SwitchonBuilding_Handler_Enum-Width (Variables|Default|GetBuilding%20Width)
    (:NewEnumerator0
      (Variables|Default|SetWidth 1))
    (:NewEnumerator1
      (Variables|Default|SetWidth 2))
    (:NewEnumerator2
      (Variables|Default|SetWidth 3))
    (:NewEnumerator3
      (Variables|Default|SetWidth 4))
    (:NewEnumerator4
      (Variables|Default|SetWidth 5))
    (:NewEnumerator5
      (Variables|Default|SetWidth 6))
    (:NewEnumerator6
      (Variables|Default|SetWidth 7))
    (:NewEnumerator7
      (Variables|Default|SetWidth 8))
    (:NewEnumerator8
      (Variables|Default|SetWidth 9))
    (:NewEnumerator9
      (Variables|Default|SetWidth 10)))
  (switch Utilities|FlowControl|Switch|SwitchonBuilding_Handler_Enum-Height (Variables|Default|GetBuilding%20Height)
    (:NewEnumerator0
      (Variables|Default|SetHeight 1))
    (:NewEnumerator1
      (Variables|Default|SetHeight 2))
    (:NewEnumerator2
      (Variables|Default|SetHeight 3))
    (:NewEnumerator3
      (Variables|Default|SetHeight 4))
    (:NewEnumerator4
      (Variables|Default|SetHeight 5))
    (:NewEnumerator5
      (Variables|Default|SetHeight 6))
    (:NewEnumerator6
      (Variables|Default|SetHeight 7))
    (:NewEnumerator7
      (Variables|Default|SetHeight 8))
    (:NewEnumerator8
      (Variables|Default|SetHeight 9))
    (:NewEnumerator9
      (Variables|Default|SetHeight 10)))
  (switch Utilities|FlowControl|Switch|SwitchonBuilding_Handler_Enum-Depth (Variables|Default|GetBuilding%20Depth)
    (:NewEnumerator0
      (Variables|Default|SetDepth 1))
    (:NewEnumerator1
      (Variables|Default|SetDepth 2))
    (:NewEnumerator2
      (Variables|Default|SetDepth 3))
    (:NewEnumerator3
      (Variables|Default|SetDepth 4))
    (:NewEnumerator4
      (Variables|Default|SetDepth 5))
    (:NewEnumerator5
      (Variables|Default|SetDepth 6))
    (:NewEnumerator6
      (Variables|Default|SetDepth 7))
    (:NewEnumerator7
      (Variables|Default|SetDepth 8))
    (:NewEnumerator8
      (Variables|Default|SetDepth 9))
    (:NewEnumerator9
      (Variables|Default|SetDepth 10)))
  (switch Utilities|FlowControl|Switch|SwitchonBuilding_Handler_Enum-Num_Sides (Variables|Default|GetNumber%20Of%20Sides)
    (:NewEnumerator0
      (Variables|Default|SetSides 1))
    (:NewEnumerator1
      (Variables|Default|SetSides 2))
    (:NewEnumerator2
      (Variables|Default|SetSides 3))
    (:NewEnumerator3
      (Variables|Default|SetSides 4))))

(fn HandleBuildingRepositioning
  (bind _building (Variables|Default|GetBuilding))
  (bind _output (Utilities|Array|Get(acopy) _building))
  (bind _building_mesh (Variables|/Game/Blueprints/Building_Unit.Building_Unit_C|GetBuilding%20Mesh _output))
  (bind _returnvalue (Transformation|GetWorldLocation _building_mesh))
  (for _index (range 0 (- (Utilities|Array|Length _building) 1))
    (bind _output_get (LocalVariables|SetIndex _index))
    (bind (_functional_index _side_base_index _previous_corner_index _side _top_corner) (CallFunction|GetFunctionalIndex _output_get))
    (LocalVariables|SetFunctional%20Index _functional_index)
    (LocalVariables|SetSide%20Base%20Index _side_base_index)
    (LocalVariables|SetPrevious%20Corner%20Index _previous_corner_index)
    (LocalVariables|SetSide _side)
    (LocalVariables|SetTop%20Corner _top_corner)
    (if (== (Math|Integer|%(Integer) (LocalVariables|GetSide) 2) 0)
      (LocalVariables|SetMultiplier (Variables|Default|GetWidth))
      (else
        (LocalVariables|SetMultiplier (Variables|Default|GetDepth))))
    (if (and (== (LocalVariables|GetFunctional%20Index) 0) (!= (LocalVariables|GetSide%20Base%20Index) 0))
      ;[1 1 1] Position The First Unit Of A New Side
      (Transformation|SetWorldRotation (Variables|/Script/Engine.Actor|GetRootComponent (Utilities|Array|Get(acopy) (Variables|Default|GetBuilding) (LocalVariables|GetIndex))) (Math|Rotator|MakeRotator (.roll (Transformation|GetWorldRotation (Variables|/Script/Engine.Actor|GetRootComponent (Utilities|Array|Get(acopy) (Variables|Default|GetBuilding) (LocalVariables|GetPrevious%20Corner%20Index))))) (.pitch (Transformation|GetWorldRotation (Variables|/Script/Engine.Actor|GetRootComponent (Utilities|Array|Get(acopy) (Variables|Default|GetBuilding) (LocalVariables|GetPrevious%20Corner%20Index))))) (- (.yaw (Transformation|GetWorldRotation (Variables|/Script/Engine.Actor|GetRootComponent (Utilities|Array|Get(acopy) (Variables|Default|GetBuilding) (LocalVariables|GetPrevious%20Corner%20Index))))) 9e+01)) false false)
      (Transformation|SetWorldLocation (Variables|/Script/Engine.Actor|GetRootComponent (Utilities|Array|Get(acopy) (Variables|Default|GetBuilding) (LocalVariables|GetIndex))) (Math|Vector|MakeVector (+ (* (Math|Trig|Cos(Degrees) (- (.yaw (Transformation|GetWorldRotation (Variables|/Script/Engine.Actor|GetRootComponent (Utilities|Array|Get(acopy) (Variables|Default|GetBuilding) (LocalVariables|GetPrevious%20Corner%20Index))))) 45.0)) 848.528137) (.x (Transformation|GetWorldLocation (Variables|/Script/Engine.Actor|GetRootComponent (Utilities|Array|Get(acopy) (Variables|Default|GetBuilding) (LocalVariables|GetPrevious%20Corner%20Index)))))) (+ (* (Math|Trig|Sin(Degrees) (- (.yaw (Transformation|GetWorldRotation (Variables|/Script/Engine.Actor|GetRootComponent (Utilities|Array|Get(acopy) (Variables|Default|GetBuilding) (LocalVariables|GetPrevious%20Corner%20Index))))) 45.0)) 848.528137) (.y (Transformation|GetWorldLocation (Variables|/Script/Engine.Actor|GetRootComponent (Utilities|Array|Get(acopy) (Variables|Default|GetBuilding) (LocalVariables|GetPrevious%20Corner%20Index)))))) (.z (Transformation|GetWorldLocation (Variables|/Script/Engine.Actor|GetRootComponent (Utilities|Array|Get(acopy) (Variables|Default|GetBuilding) (LocalVariables|GetPrevious%20Corner%20Index)))))) false false)
      (else
        ;[1 1 1] Position The Current Unit
        (Transformation|SetWorldRotation (Variables|/Script/Engine.Actor|GetRootComponent (Utilities|Array|Get(acopy) (Variables|Default|GetBuilding) (LocalVariables|GetIndex))) (Math|Rotator|MakeRotator (.roll (Transformation|GetWorldRotation (Variables|/Game/Blueprints/Building_Unit.Building_Unit_C|GetRoof%20Mesh (Utilities|Array|Get(acopy) (Variables|Default|GetBuilding) (LocalVariables|GetSide%20Base%20Index))))) 0.0 (.yaw (Transformation|GetWorldRotation (Variables|/Game/Blueprints/Building_Unit.Building_Unit_C|GetRoof%20Mesh (Utilities|Array|Get(acopy) (Variables|Default|GetBuilding) (LocalVariables|GetSide%20Base%20Index)))))) false false)
        (Transformation|SetWorldLocation (Variables|/Script/Engine.Actor|GetRootComponent (Utilities|Array|Get(acopy) (Variables|Default|GetBuilding) (LocalVariables|GetIndex))) (Math|Vector|MakeVector (+ (* (Math|Integer|%(Integer) (LocalVariables|GetFunctional%20Index) (LocalVariables|GetMultiplier)) (* (Math|Trig|Cos(Degrees) (.yaw (Transformation|GetWorldRotation (Variables|/Game/Blueprints/Building_Unit.Building_Unit_C|GetRoof%20Mesh (Utilities|Array|Get(acopy) (Variables|Default|GetBuilding) (LocalVariables|GetSide%20Base%20Index)))))) 1.2e+03)) (.x (Transformation|GetWorldLocation (Variables|/Game/Blueprints/Building_Unit.Building_Unit_C|GetRoof%20Mesh (Utilities|Array|Get(acopy) (Variables|Default|GetBuilding) (LocalVariables|GetSide%20Base%20Index)))))) (+ (* (Math|Integer|%(Integer) (LocalVariables|GetFunctional%20Index) (LocalVariables|GetMultiplier)) (* (Math|Trig|Sin(Degrees) (.yaw (Transformation|GetWorldRotation (Variables|/Game/Blueprints/Building_Unit.Building_Unit_C|GetRoof%20Mesh (Utilities|Array|Get(acopy) (Variables|Default|GetBuilding) (LocalVariables|GetSide%20Base%20Index)))))) 1.2e+03)) (.y (Transformation|GetWorldLocation (Variables|/Game/Blueprints/Building_Unit.Building_Unit_C|GetRoof%20Mesh (Utilities|Array|Get(acopy) (Variables|Default|GetBuilding) (LocalVariables|GetSide%20Base%20Index)))))) (+ (.z (Transformation|GetWorldLocation (Variables|/Game/Blueprints/Building_Unit.Building_Unit_C|GetRoof%20Mesh (Utilities|Array|Get(acopy) (Variables|Default|GetBuilding) (LocalVariables|GetSide%20Base%20Index))))) (* (/ (LocalVariables|GetFunctional%20Index) (LocalVariables|GetMultiplier)) 4e+02))) false false)))
    ;[1 1 1] Only Place Roofs On Top Floor, Excluding First Corner Piece To Prevent Duplicates
    (if (and (!= (LocalVariables|GetIndex) (LocalVariables|GetTop%20Corner)) (== (/ (LocalVariables|GetFunctional%20Index) (LocalVariables|GetMultiplier)) (- (Variables|Default|GetHeight) 1)))
      (bind _output_get_2 (Variables|/Game/Blueprints/Building_Unit.Building_Unit_C|SetToggle%20Roof (Utilities|Array|Get(acopy) (Variables|Default|GetBuilding) (LocalVariables|GetIndex)) true))
      (Rendering|SetVisibility (Variables|/Game/Blueprints/Building_Unit.Building_Unit_C|GetRoof%20Mesh (Utilities|Array|Get(acopy) (Variables|Default|GetBuilding) (LocalVariables|GetIndex))) _output_get_2 false)
      (else
        (bind _output_get_3 (Variables|/Game/Blueprints/Building_Unit.Building_Unit_C|SetToggle%20Roof (Utilities|Array|Get(acopy) (Variables|Default|GetBuilding) (LocalVariables|GetIndex)) false))
        (Rendering|SetVisibility (Variables|/Game/Blueprints/Building_Unit.Building_Unit_C|GetRoof%20Mesh (Utilities|Array|Get(acopy) (Variables|Default|GetBuilding) (LocalVariables|GetIndex))) _output_get_3 false))))
  ;[1 1 1] Reposition Building Handler
  (Transformation|SetWorldLocation (Variables|Default|GetDefaultSceneRoot) (Math|Vector|MakeVector (.x _returnvalue) (.y _returnvalue) (+ (.z _returnvalue) (* (+ (Variables|Default|GetHeight) 2) 4e+02))) false false))

(fn RandomizeBuildingUnitDetails
  (bind _building (Variables|Default|GetBuilding))
  (for _index (range 0 (- (Utilities|Array|Length _building) 1))
    (bind _output_get (Variables|/Game/Blueprints/Building_Unit.Building_Unit_C|SetToggle%20Awning (Utilities|Array|Get(acopy) _building _index) (Math|Random|RandomBoolwithWeight 0.5)))
    (Rendering|SetVisibility (Variables|/Game/Blueprints/Building_Unit.Building_Unit_C|GetAwning%20Mesh (Utilities|Array|Get(acopy) _building _index)) _output_get false)
    (bind _output_get_2 (Variables|/Game/Blueprints/Building_Unit.Building_Unit_C|SetToggle%20Rails%20-%20Front (Utilities|Array|Get(acopy) _building _index) (Math|Random|RandomBoolwithWeight 0.5)))
    (Rendering|SetVisibility (Variables|/Game/Blueprints/Building_Unit.Building_Unit_C|GetFront%20Rail%20Mesh (Utilities|Array|Get(acopy) _building _index)) _output_get_2 false)
    (bind _output_get_3 (Variables|/Game/Blueprints/Building_Unit.Building_Unit_C|SetToggle%20Rails%20-%20Side (Utilities|Array|Get(acopy) _building _index) (Math|Random|RandomBoolwithWeight 0.5)))
    (Rendering|SetVisibility (Variables|/Game/Blueprints/Building_Unit.Building_Unit_C|GetSide%20Rail%20Mesh (Utilities|Array|Get(acopy) _building _index)) _output_get_3 false)
    (CallFunction|HandleVentRandomization _index)))

(fn HandleVentRandomization
  (params (Index :type Integer))
  (bind _building (Variables|Default|GetBuilding))
  (bind _output (Utilities|Array|Get(acopy) _building Index))
  (bind _vent_1_mesh (Variables|/Game/Blueprints/Building_Unit.Building_Unit_C|GetVent%201%20Mesh _output))
  (Variables|/Game/Blueprints/Building_Unit.Building_Unit_C|SetToggle%20Vent%20-%201 _output false)
  (Variables|/Game/Blueprints/Building_Unit.Building_Unit_C|SetToggle%20Vent%20-%202 _output false)
  (Variables|/Game/Blueprints/Building_Unit.Building_Unit_C|SetToggle%20Vent%20-%203 _output false)
  (Variables|/Game/Blueprints/Building_Unit.Building_Unit_C|SetToggle%20Vent%20-%204 _output false)
  (Variables|/Game/Blueprints/Building_Unit.Building_Unit_C|SetToggle%20Vent%20-%205 _output false)
  (Rendering|SetVisibility _vent_1_mesh false false)
  (switch int (Math|Random|RandomIntegerinRange 0 5)
    (:0
      (Variables|/Game/Blueprints/Building_Unit.Building_Unit_C|SetVent%20Selection _output "NewEnumerator5"))
    (:1
      (Variables|/Game/Blueprints/Building_Unit.Building_Unit_C|SetVent%20Selection _output "NewEnumerator0")
      (Rendering|SetVisibility _vent_1_mesh true false)
      (Variables|/Game/Blueprints/Building_Unit.Building_Unit_C|SetToggle%20Vent%20-%201 _output true))
    (:2
      (Variables|/Game/Blueprints/Building_Unit.Building_Unit_C|SetVent%20Selection _output "NewEnumerator1")
      (Rendering|SetVisibility (Variables|/Game/Blueprints/Building_Unit.Building_Unit_C|GetVent%202%20Mesh _output) true false)
      (Variables|/Game/Blueprints/Building_Unit.Building_Unit_C|SetToggle%20Vent%20-%202 _output true))
    (:3
      (Variables|/Game/Blueprints/Building_Unit.Building_Unit_C|SetVent%20Selection _output "NewEnumerator2")
      (Rendering|SetVisibility (Variables|/Game/Blueprints/Building_Unit.Building_Unit_C|GetVent%203%20Mesh _output) true false)
      (Variables|/Game/Blueprints/Building_Unit.Building_Unit_C|SetToggle%20Vent%20-%203 _output true))
    (:4
      (Variables|/Game/Blueprints/Building_Unit.Building_Unit_C|SetVent%20Selection _output "NewEnumerator3")
      (Rendering|SetVisibility (Variables|/Game/Blueprints/Building_Unit.Building_Unit_C|GetVent%204%20Mesh _output) true false)
      (Variables|/Game/Blueprints/Building_Unit.Building_Unit_C|SetToggle%20Vent%20-%204 _output true))
    (:5
      (Variables|/Game/Blueprints/Building_Unit.Building_Unit_C|SetVent%20Selection _output "NewEnumerator4")
      (Rendering|SetVisibility (Variables|/Game/Blueprints/Building_Unit.Building_Unit_C|GetVent%205%20Mesh _output) true false)
      (Variables|/Game/Blueprints/Building_Unit.Building_Unit_C|SetToggle%20Vent%20-%205 _output true))))

(fn GetFunctionalIndex
  (params (Index :type Integer))
  (bind _height (Variables|Default|GetHeight))
  (bind _height_2 (Variables|Default|GetHeight))
  (bind _depth (Variables|Default|GetDepth))
  (bind _width (Variables|Default|GetWidth))
  (bind _returnvalue (* _depth _height))
  (bind _returnvalue_2 (* _width _height_2))
  (LocalVariables|SetCurrent%20Index Index)
  (LocalVariables|SetBase%20Index 0)
  (LocalVariables|SetCorner%20Index 0)
  (LocalVariables|SetCurrent%20Side 0)
  (LocalVariables|SetTop%20Corner%20Unit -1)
  ;[1 1 1] Check If The Current Building Unit Is On The First Or Third Wall
  (if (< (LocalVariables|GetCurrent%20Index) _returnvalue_2) :!label _label
    _
    (else
      (LocalVariables|SetCurrent%20Index (- (LocalVariables|GetCurrent%20Index) _returnvalue_2))
      (LocalVariables|SetCorner%20Index (+ (- (Variables|Default|GetWidth) 1) (LocalVariables|GetBase%20Index)))
      (LocalVariables|SetBase%20Index (+ (LocalVariables|GetBase%20Index) _returnvalue_2))
      (LocalVariables|SetTop%20Corner%20Unit (+ (LocalVariables|GetBase%20Index) (* (Variables|Default|GetDepth) (- (Variables|Default|GetHeight) 1))))
      (Math|Integer|IncrementInt (LocalVariables|GetCurrent%20Side)
        (:%20%20
          ;[1 1 1] Check If The Current Building Unit Is On The Second Or Fourth Wall
          (if (< (LocalVariables|GetCurrent%20Index) _returnvalue)
            _
            (else
              (LocalVariables|SetCurrent%20Index (- (LocalVariables|GetCurrent%20Index) _returnvalue))
              (LocalVariables|SetCorner%20Index (+ (- (Variables|Default|GetDepth) 1) (LocalVariables|GetBase%20Index)))
              (LocalVariables|SetBase%20Index (+ (LocalVariables|GetBase%20Index) _returnvalue))
              (LocalVariables|SetTop%20Corner%20Unit (+ (LocalVariables|GetBase%20Index) (* (Variables|Default|GetWidth) (- (Variables|Default|GetHeight) 1))))
              (Math|Integer|IncrementInt (LocalVariables|GetCurrent%20Side)
                (:%20%20
                  (goto _label)))))))))
  (return (LocalVariables|GetCurrent%20Index) (LocalVariables|GetBase%20Index) (LocalVariables|GetCorner%20Index) (LocalVariables|GetCurrent%20Side) (LocalVariables|GetTop%20Corner%20Unit)))