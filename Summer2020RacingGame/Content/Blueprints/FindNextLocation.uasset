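; Behavior tree task that picks the next spline point along a HoverSedan's track as its destination.
; It steps the car's current point forwards or backwards according to its direction flag, wrapping at either end of the spline.
; It snaps the car's rotation from the previous point toward the new one, then writes that point plus the car's offset to a blackboard vector.
; Pawns that are not HoverSedans abort the task.
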(event EventReceiveExecuteAI
  (params (OwnerController :type AI%20Controller%20Object%20Reference) (ControlledPawn :type Pawn%20Object%20Reference))
  (bind _ashover_sedan (Utilities|Casting|CastToHoverSedan ControlledPawn)
    (:then
      (bind _output_get (Variables|Default|SetStarting%20Location (Spline|GetLocationatSplinePoint (Variables|/Game/Blueprints/TrackGenerator.TrackGenerator_C|GetSpline (Variables|/Game/Blueprints/HoverSedan.HoverSedan_C|GetTrack _ashover_sedan)) (Variables|/Game/Blueprints/HoverSedan.HoverSedan_C|GetCurrent%20Point _ashover_sedan) "World")))
      (if (Variables|/Game/Blueprints/HoverSedan.HoverSedan_C|GetForwards _ashover_sedan)
        (bind _result (Math|Integer|IncrementInt (Variables|/Game/Blueprints/HoverSedan.HoverSedan_C|GetCurrent%20Point _ashover_sedan))
          (:%20%20
            (if (== (Variables|/Game/Blueprints/TrackGenerator.TrackGenerator_C|GetNumSplinePoints (Variables|/Game/Blueprints/HoverSedan.HoverSedan_C|GetTrack _ashover_sedan)) _result)
              (Variables|/Game/Blueprints/HoverSedan.HoverSedan_C|SetCurrent%20Point _ashover_sedan 0))))
        (else
          (bind _result_2 (Math|Integer|DecrementInt (Variables|/Game/Blueprints/HoverSedan.HoverSedan_C|GetCurrent%20Point _ashover_sedan))
            (:%20%20
              (if (== _result_2 -1)
                (Variables|/Game/Blueprints/HoverSedan.HoverSedan_C|SetCurrent%20Point _ashover_sedan (- (Variables|/Game/Blueprints/TrackGenerator.TrackGenerator_C|GetNumSplinePoints (Variables|/Game/Blueprints/HoverSedan.HoverSedan_C|GetTrack _ashover_sedan)) 1)))))))
      (Transformation|SetActorRotation _ashover_sedan (Math|Rotator|FindLookatRotation _output_get (Spline|GetLocationatSplinePoint (Variables|/Game/Blueprints/TrackGenerator.TrackGenerator_C|GetSpline (Variables|/Game/Blueprints/HoverSedan.HoverSedan_C|GetTrack _ashover_sedan)) (Variables|/Game/Blueprints/HoverSedan.HoverSedan_C|GetCurrent%20Point _ashover_sedan) "World")))
      (AI|BehaviorTree|SetBlackboardValueasVector (Variables|Default|GetVector) (+ (Spline|GetLocationatSplinePoint (Variables|/Game/Blueprints/TrackGenerator.TrackGenerator_C|GetSpline (Variables|/Game/Blueprints/HoverSedan.HoverSedan_C|GetTrack _ashover_sedan)) (Variables|/Game/Blueprints/HoverSedan.HoverSedan_C|GetCurrent%20Point _ashover_sedan) "World") (Variables|/Game/Blueprints/HoverSedan.HoverSedan_C|GetOffset _ashover_sedan)))
      (AI|BehaviorTree|FinishExecute true))
    (:CastFailed
      (Class|BTTaskBlueprintBase|FinishAbort))))