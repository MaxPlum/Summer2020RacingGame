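; Configurable apartment building actor with optional awning, rail and vent detail meshes.
; The construction script shows or hides each detail from its toggle and assigns a material instance to every mesh, building included, from a per-mesh Red/Blue/Green texture enum.
; On BeginPlay, collision is disabled on any detail that is toggled off.
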(event EventBeginPlay
  ;[1 1 1] Set Collision To None If Detail Is Not Visible
  (CallFunction|UpdateCollision (Variables|Default|GetAwningMesh) (Variables|Visibility|GetToggle%20Awning))
  (CallFunction|UpdateCollision (Variables|Default|GetRailsMesh) (Variables|Visibility|GetToggle%20Rails))
  (CallFunction|UpdateCollision (Variables|Default|GetVentMesh) (Variables|Visibility|GetToggle%20Vent)))

(event Collision|EventActorBeginOverlap
  (params (OtherActor :type Actor%20Object%20Reference)))

(event EventTick
  (params (DeltaSeconds :type Float%20%28single-precision%29)))

(fn ConstructionScript
  ;[1 1 1] Toggle Component Visibility And Collision
  (Rendering|SetVisibility (Variables|Default|GetAwningMesh) (Variables|Visibility|GetToggle%20Awning) false)
  (Rendering|SetVisibility (Variables|Default|GetRailsMesh) (Variables|Visibility|GetToggle%20Rails) false)
  (Rendering|SetVisibility (Variables|Default|GetVentMesh) (Variables|Visibility|GetToggle%20Vent) false)
  ;[1 1 1] Set Object Texture
  (CallFunction|UpdateTexture-Apartment (Variables|Default|GetBuildingMesh) (Variables|Texture|GetBuilding%20Texture))
  (CallFunction|UpdateTexture-Apartment (Variables|Default|GetAwningMesh) (Variables|Texture|GetAwning%20Texture))
  (CallFunction|UpdateTexture-Apartment (Variables|Default|GetRailsMesh) (Variables|Texture|GetRails%20Texture))
  (CallFunction|UpdateTexture-Apartment (Variables|Default|GetVentMesh) (Variables|Texture|GetVent%20Texture)))

(fn UpdateCollision
  (params (Mesh :type Static%20Mesh%20Component%20Object%20Reference) (Toggle :type Boolean))
  (if (not Toggle)
    (Collision|SetCollisionEnabled Mesh "NoCollision")))

(fn UpdateTexture-Apartment
  (params (Mesh :type Static%20Mesh%20Component%20Object%20Reference) (Texture%20Enum :type Texture_Enum-Apartment%20Enum :default "NewEnumerator0"))
  (switch Utilities|FlowControl|Switch|SwitchonTexture_Enum-Apartment Texture%20Enum
    (:NewEnumerator0
      (Rendering|Material|SetMaterial Mesh 0 "/Game/Architecture/Buildings/Materials/M_Building_Master_Inst.M_Building_Master_Inst"))
    (:NewEnumerator1
      (Rendering|Material|SetMaterial Mesh 0 "/Game/Architecture/Buildings/Materials/M_Awning_Master_Inst.M_Awning_Master_Inst"))
    (:NewEnumerator2
      (Rendering|Material|SetMaterial Mesh 0 "/Game/Architecture/Buildings/Materials/M_Rails_Master_Inst.M_Rails_Master_Inst"))))