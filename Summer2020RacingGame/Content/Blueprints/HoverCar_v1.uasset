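; Physics-driven hover car that the player accelerates, reverses and steers through forces and torques on its mesh, with turning inverted when reversing.
; BeginPlay initializes six hover components, including two angled front ones, and two floor sensors on the mesh.
; Each tick averages the sensors' floor normals to apply surface-relative gravity, falling back to world down without hits.
; An unfinished self-righting torque is left disconnected.
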(event EventBeginPlay
  (bind _sensorcomponentcenter (Variables|Default|GetSensorComponentCenter))
  (bind _sensor_array (Variables|Default|GetSensor%20Array))
  (bind _carmesh (Variables|Default|GetCarMesh))
  ;[1 1 1] Initialize Hover Components
  (Default|InitializeHoverComponent (Variables|Default|GetHoverComponentFrontRight) _carmesh)
  (Default|InitializeSensorComponent _sensorcomponentcenter _carmesh)
  (Utilities|Array|AddUnique _sensor_array _sensorcomponentcenter)
  (Utilities|Array|AddUnique _sensor_array (Variables|Default|GetSensorComponentCenter1)))

(event EventTick
  (params (DeltaSeconds :type Float%20%28single-precision%29))
  (Variables|Default|SetSensor%20Hits 0)
  (Variables|Default|SetGravity%20Vector "0, 0, 0")
  (for _array_element (Variables|Default|GetSensor%20Array)
    (CallFunction|CalculateGravityVector _array_element))
  (if (== (Variables|Default|GetSensor%20Hits) 0)
    (Variables|Default|SetGravity%20Vector "0, 0,1.000000")
    (else
      (Variables|Default|SetGravity%20Vector (/ (Variables|Default|GetGravity%20Vector) (Variables|Default|GetSensor%20Hits)))))
  (Physics|AddForce (Variables|Default|GetCarMesh) (* (Variables|Default|GetGravity%20Vector) (* -1 (Variables|Default|GetGravity))) "None" false))

(event Input|AxisEvents|InputAxisMoveForward
  (params (AxisValue :type Float%20%28single-precision%29))
  ;[1 1 1] Handle Forward/Backward Movement
  (bind _output_get (Variables|Default|SetMovement%20Input AxisValue))
  (Physics|AddForce (Variables|Default|GetCarMesh) (* (* (* (Math|Vector|GetForwardVector (Variables|Default|GetCarMesh)) (Variables|Default|GetAcceleration)) _output_get) (Math|Float|SelectFloat (Variables|Default|GetForward%20Acceleration%20Percentage) (Variables|Default|GetReverse%20Acceleration%20Percentage) (>= AxisValue 0.0))) "None" false))

(event Input|AxisEvents|InputAxisMoveRight
  (params (AxisValue :type Float%20%28single-precision%29))
  (bind _carmesh (Variables|Default|GetCarMesh))
  ;[1 1 1] Handle Turning
  (bind _returnvalue (Physics|GetPhysicsLinearVelocity (Variables|Default|GetCarMesh) "None"))
  (Class|PrimitiveComponent|AddTorqueinRadians _carmesh (* (Math|Vector|GetUpVector _carmesh) (* (Math|Float|SelectFloat -1.0 1.0 (< (Variables|Default|GetMovement%20Input) 0.0)) (* AxisValue (Variables|Default|GetTurning%20Velocity)))) "None" false))

(fn ConstructionScript)

(fn CalculateGravityVector
  (params (Sensor%20Component :type Sensor%20Component%20Object%20Reference))
  (bind (_surface_hit _floor_normal) (Default|GetFloorNormal Sensor%20Component))
  (if _surface_hit
    (Variables|Default|SetGravity%20Vector (+ _floor_normal (Variables|Default|GetGravity%20Vector)))
    (Math|Integer|IncrementInt (Variables|Default|GetSensor%20Hits))))