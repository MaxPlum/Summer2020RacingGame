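; Spline-driven track generator actor that builds a road with optional guard rails from editable spline points in the construction script.
; Per-point data sets mesh, bank, width and thickness for each spline mesh segment, while active branches redirect segments to other points and LoopTrack closes the circuit.
; It also spawns and repositions attached TrackObjects, can label point numbers, and destroys itself below two points.
; A flag-triggered event resamples the spline at fixed spacing with computed custom tangents.
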(event Custom|Spawn%20Track%20Objects
  (bind _track_objects (Variables|Default|GetTrack%20Objects))
  (for (_array_element _array_index) _track_objects
    (Utilities|IsValid _array_element
      (:Is%20Not%20Valid
        (bind _returnvalue (Game|SpawnActorfromClass "/Game/Blueprints/TrackObject.TrackObject_C" (Transformation|GetWorldTransform (Variables|Default|GetSpline)) "AlwaysSpawn" 0 0))
        (Variables|/Game/Blueprints/TrackObject.TrackObject_C|SetParent%20chungus _returnvalue self)
        (Utilities|Array|SetArrayElem _track_objects _array_index _returnvalue)))))

(event Custom|CustomEvent_0
  (bind _newvar_2 (Variables|Default|GetNewVar_2))
  (bind _newvar_1 (Variables|Default|GetNewVar_1))
  (bind _spline (Variables|Default|GetSpline))
  (bind _newvar_1_2 (Variables|Default|GetNewVar_1))
  (bind _spline_2 (Variables|Default|GetSpline))
  (if (Variables|Default|GetNewVar_0)
    (bind _returnvalue (Game|SpawnActorfromClass "/Game/Blueprints/TrackObject.TrackObject_C" (Transformation|GetWorldTransform (Variables|Default|GetSpline)) "AlwaysSpawn" 0 0))
    (Utilities|IsValid _returnvalue
      (:Is%20Valid
        (Actor|DestroyActor _returnvalue)
        (Variables|Default|SetNewVar_0 false)
        (Utilities|FlowControl|Sequence
          (:then_0
            (Variables|Default|SetNewVar_4 0.0)
            (if (< (Variables|Default|GetNewVar_4) (Spline|GetDistanceAlongSplineatSplinePoint _spline_2 (- (Spline|GetNumberOfSplinePoints _spline_2) 1))) :!label _label
              (if (== (Variables|Default|GetNewVar_4) 0.0)
                (Utilities|Array|Add _newvar_1_2 (.location (Spline|GetTransformatDistanceAlongSpline _spline (Variables|Default|GetNewVar_4) "Local" false)))
                (else
                  (Utilities|Array|Add _newvar_1_2 (.location (Spline|GetTransformatDistanceAlongSpline _spline (- (Variables|Default|GetNewVar_4) 5e+01) "Local" false)))))
              (Utilities|Array|Add (Variables|Default|GetNewVar_2) (.location (Spline|GetTransformatDistanceAlongSpline _spline (Variables|Default|GetNewVar_4) "Local" false)))
              (Utilities|Array|Add _newvar_1_2 (.location (Spline|GetTransformatDistanceAlongSpline _spline (+ (Variables|Default|GetNewVar_4) 5e+01) "Local" false)))
              (Variables|Default|SetNewVar_4 (+ (Variables|Default|GetNewVar_4) (Variables|Default|GetNewVar_3)))
              (goto _label)
              (else
                (Spline|ClearSplinePoints _spline true))))
          (:then_1
            (for (_array_element _array_index) _newvar_2
              (bind (_newparam2 _newparam3) (CallFunction|NewFunction1 _newvar_1 _newvar_2 _array_index))
              (Class|SplineComponent|AddPoint _spline (Utilities|Struct|MakeSplinePoint (Math|Conversions|ToFloat(Integer) _array_index) _array_element _newparam2 _newparam3 "0.000000,0.000000,0.000000" "1.000000,1.000000,1.000000" "CurveCustomTangent") true))
            (Utilities|Array|Clear _newvar_2)
            (Utilities|Array|Clear _newvar_1)))))))

(event EventBeginPlay)

(event Collision|EventActorBeginOverlap
  (params (OtherActor :type Actor%20Object%20Reference)))

(event EventTick
  (params (DeltaSeconds :type Float%20%28single-precision%29)))

(fn ConstructionScript
  (Utilities|FlowControl|Sequence
    (:then_0
      (Spline|GetNumberOfSplinePoints))
    (:then_2
      (|CheckTrackObjects))
    (:then_3
      (|BuildTrackDataArray))
    (:then_5
      (|ConstructionLoop)
      (|StoreDrawLeftRightGuardRail)
      (|BoolDrawLeftRight))
    (:then_6
      (|DrawTrackPointNumber))
    (:then_7
      (|DeleteSplineIfTooSmall))
    (:then_8
      (CallFunction|CustomEvent0))))

(fn BuildTrackElement
  (params (Loop%20Index :type Integer) (Destination%20Index :type Integer) (Track%20Element%20Mesh :type Track_Mesh_Drawing_Enum%20Enum :default "NewEnumerator0"))
  (LocalVariables|SetLocal_CurrentLoopIndex Loop%20Index)
  (LocalVariables|SetLocal_NextLoopIndex Destination%20Index)
  (switch Utilities|FlowControl|Switch|SwitchonTrack_Mesh_Drawing_Enum Track%20Element%20Mesh
    (:NewEnumerator0
      (switch Utilities|FlowControl|Switch|SwitchonTrack_Mesh_Enum (.trackmesh (Utilities|Array|Get(acopy) (Variables|TrackSetup|GetTrackDataArray) (LocalVariables|GetLocal_CurrentLoopIndex)))
        (:NewEnumerator0
          (LocalVariables|SetLocal_TrackElementMesh (Variables|TrackMeshes|GetTrackMesh%20-%20Low%20Poly)))
        (:NewEnumerator1
          (LocalVariables|SetLocal_TrackElementMesh (Variables|TrackMeshes|GetTrackMesh%20-%20Mid%20Poly)))))
    (:NewEnumerator1
      (LocalVariables|SetLocal_TrackElementMesh (Variables|TrackMeshes|GetLeftGuardRailMesh)))
    (:NewEnumerator2
      (LocalVariables|SetLocal_TrackElementMesh (Variables|TrackMeshes|GetRightGuardRailMesh))))
  (Utilities|FlowControl|Sequence
    (:then_0
      (LocalVariables|SetLocal_StartLocation (.Location (Spline|GetLocationandTangentatSplinePoint (Variables|Default|GetSpline) (LocalVariables|GetLocal_CurrentLoopIndex) "Local")))
      (LocalVariables|SetLocal_StartTangent (.Tangent (Spline|GetLocationandTangentatSplinePoint (Variables|Default|GetSpline) (LocalVariables|GetLocal_CurrentLoopIndex) "Local")))
      (LocalVariables|SetLocal_EndLocation (.Location (Spline|GetLocationandTangentatSplinePoint (Variables|Default|GetSpline) (LocalVariables|GetLocal_NextLoopIndex) "Local")))
      (LocalVariables|SetLocalEndTangent (.Tangent (Spline|GetLocationandTangentatSplinePoint (Variables|Default|GetSpline) (LocalVariables|GetLocal_NextLoopIndex) "Local")))
      (LocalVariables|SetLocal_StartRoll (.trackbank (Utilities|Array|Get(acopy) (Variables|TrackSetup|GetTrackDataArray) (LocalVariables|GetLocal_CurrentLoopIndex))))
      (LocalVariables|SetLocal_StartScale (Math|Vector2D|MakeVector2D (.trackwidth (Utilities|Array|Get(acopy) (Variables|TrackSetup|GetTrackDataArray) (LocalVariables|GetLocal_CurrentLoopIndex))) (.trackthickness (Utilities|Array|Get(acopy) (Variables|TrackSetup|GetTrackDataArray) (LocalVariables|GetLocal_CurrentLoopIndex)))))
      (LocalVariables|SetLocal_EndRoll (.trackbank (Utilities|Array|Get(acopy) (Variables|TrackSetup|GetTrackDataArray) (LocalVariables|GetLocal_NextLoopIndex))))
      (LocalVariables|SetLocal_EndScale (Math|Vector2D|MakeVector2D (.trackwidth (Utilities|Array|Get(acopy) (Variables|TrackSetup|GetTrackDataArray) (LocalVariables|GetLocal_NextLoopIndex))) (.trackthickness (Utilities|Array|Get(acopy) (Variables|TrackSetup|GetTrackDataArray) (LocalVariables|GetLocal_NextLoopIndex))))))
    (:then_1
      (bind _returnvalue (AddComponent|AddSplineMeshComponent false))
      (LocalVariables|SetLocal_CurrentSplineMesh _returnvalue)
      (Components|StaticMesh|SetStaticMesh (LocalVariables|GetLocal_CurrentSplineMesh) (LocalVariables|GetLocal_TrackElementMesh))
      (SplineMesh|SetStartandEnd (LocalVariables|GetLocal_CurrentSplineMesh) (LocalVariables|GetLocal_StartLocation) (LocalVariables|GetLocal_StartTangent) (LocalVariables|GetLocal_EndLocation) (LocalVariables|GetLocalEndTangent) true :!class /Script/Engine.SplineMeshComponent)
      (Class|SplineMeshComponent|SetStartRoll (LocalVariables|GetLocal_CurrentSplineMesh) (LocalVariables|GetLocal_StartRoll) true)
      (Class|SplineMeshComponent|SetEndRoll (LocalVariables|GetLocal_CurrentSplineMesh) (LocalVariables|GetLocal_EndRoll) true)
      (SplineMesh|SetStartScale (LocalVariables|GetLocal_CurrentSplineMesh) (LocalVariables|GetLocal_StartScale) true :!class /Script/Engine.SplineMeshComponent)
      (SplineMesh|SetEndScale (LocalVariables|GetLocal_CurrentSplineMesh) (LocalVariables|GetLocal_EndScale) true :!class /Script/Engine.SplineMeshComponent)
      (Collision|SetCollisionEnabled (LocalVariables|GetLocal_CurrentSplineMesh) (select (Variables|Debug|GetCollisions) "QueryAndPhysics" "NoCollision")))))

(fn HandleDeletedSplinePoint
  (LocalVariables|SetIndex 0)
  (if (> (Utilities|Array|Length (Variables|Default|GetSpline%20Point%20Distances)) (Variables|Default|GetNumSplinePoints)) :!label _label
    (if (!= (Utilities|Array|Get(acopy) (Variables|Default|GetSpline%20Point%20Distances) (LocalVariables|GetIndex)) (Spline|GetDistanceAlongSplineatSplinePoint (Variables|Default|GetSpline) (LocalVariables|GetIndex)))
      (Utilities|Array|RemoveIndex (Variables|Default|GetSpline%20Point%20Distances) (LocalVariables|GetIndex))
      (Utilities|Array|RemoveIndex (Variables|TrackSetup|GetTrackDataArray) (LocalVariables|GetIndex))
      (CallFunction|HandleDeletedBranch (LocalVariables|GetIndex))
      (goto _label)
      (else
        (Math|Integer|IncrementInt (LocalVariables|GetIndex)
          (:%20%20
            (goto _label)))))))

(fn HandleNewSplinePoint
  (bind _spline_point_distances (Variables|Default|GetSpline%20Point%20Distances))
  (if (== (Utilities|Array|Length _spline_point_distances) 0)
    (Utilities|Array|Add _spline_point_distances (Spline|GetDistanceAlongSplineatSplinePoint (Variables|Default|GetSpline) 0))
    (Utilities|Array|Add (Variables|TrackSetup|GetTrackDataArray) (Variables|Default|GetTrackMeshDefaults)))
  (LocalVariables|SetIndex 0)
  (LocalVariables|SetInsertion%20Index 0)
  (if (< (Utilities|Array|Length (Variables|Default|GetSpline%20Point%20Distances)) (Variables|Default|GetNumSplinePoints)) :!label _label
    (if (!= (Utilities|Array|Get(acopy) (Variables|Default|GetSpline%20Point%20Distances) (LocalVariables|GetInsertion%20Index)) (Spline|GetDistanceAlongSplineatSplinePoint (Variables|Default|GetSpline) (LocalVariables|GetIndex)))
      (Utilities|Array|Insert (Variables|Default|GetSpline%20Point%20Distances) (Spline|GetDistanceAlongSplineatSplinePoint (Variables|Default|GetSpline) (LocalVariables|GetIndex)) (LocalVariables|GetInsertion%20Index))
      (Utilities|Array|Insert (Variables|TrackSetup|GetTrackDataArray) (Variables|Default|GetTrackMeshDefaults) (LocalVariables|GetInsertion%20Index))
      (CallFunction|UpdateTrackDataArray (LocalVariables|GetInsertion%20Index))
      (CallFunction|HandleAddedBranch (LocalVariables|GetInsertion%20Index))
      (else
        (Math|Integer|IncrementInt (LocalVariables|GetIndex)
          (:%20%20
            _))))
    (Math|Integer|IncrementInt (LocalVariables|GetInsertion%20Index)
      (:%20%20
        (goto _label)))))

(fn UpdateSplinePointDistances
  (for (_ _array_index) (Variables|Default|GetSpline%20Point%20Distances)
    (Utilities|Array|SetArrayElem (Variables|Default|GetSpline%20Point%20Distances) _array_index (Spline|GetDistanceAlongSplineatSplinePoint (Variables|Default|GetSpline) _array_index))))

(fn UpdateTrackDataArray
  (params (Starting%20Index :type Integer))
  (bind _trackdataarray (Variables|TrackSetup|GetTrackDataArray))
  (LocalVariables|SetEnding%20Index Starting%20Index)
  (LocalVariables|SetIndex (- (Utilities|Array|Length (Variables|TrackSetup|GetTrackDataArray)) 1))
  (if (> (LocalVariables|GetIndex) (LocalVariables|GetEnding%20Index)) :!label _label
    (Utilities|Array|SetArrayElem _trackdataarray (LocalVariables|GetIndex) (Utilities|Array|Get(acopy) _trackdataarray (- (LocalVariables|GetIndex) 1)))
    (goto _label)))

(fn HandleDeletedBranch
  (params (Index :type Integer))
  (bind _track_branches (Variables|TrackSetup|GetTrack%20Branches))
  (bind _track_branches_2 (Variables|TrackSetup|GetTrack%20Branches))
  (LocalVariables|SetDeleted%20Index (+ Index 1))
  (for (_ _array_index) _track_branches
    (Math|Integer|CompareInt (.startingsplinepoint (Utilities|Array|Get(acopy) _track_branches _array_index)) (LocalVariables|GetDeleted%20Index)
      (:>
        (Utilities|Array|SetArrayElem _track_branches _array_index (Utilities|Struct|MakeTrackBranchData (.branchactive (Utilities|Array|Get(acopy) _track_branches _array_index)) (- (.startingsplinepoint (Utilities|Array|Get(acopy) _track_branches _array_index)) 1) (.endingsplinepoint (Utilities|Array|Get(acopy) _track_branches _array_index)) false))
        (if (> (.endingsplinepoint (Utilities|Array|Get(acopy) _track_branches _array_index)) (LocalVariables|GetDeleted%20Index)) :!label _label
          (Utilities|Array|SetArrayElem _track_branches_2 _array_index (Utilities|Struct|MakeTrackBranchData (.branchactive (Utilities|Array|Get(acopy) _track_branches_2 _array_index)) (.startingsplinepoint (Utilities|Array|Get(acopy) _track_branches_2 _array_index)) (- (.endingsplinepoint (Utilities|Array|Get(acopy) _track_branches_2 _array_index)) 1) (.removebranch (Utilities|Array|Get(acopy) _track_branches_2 _array_index))))))
      (:==
        (Utilities|Array|RemoveIndex _track_branches _array_index))
      (:<
        (goto _label)))))

(fn HandleAddedBranch
  (params (Index :type Integer))
  (bind _track_branches (Variables|TrackSetup|GetTrack%20Branches))
  (bind _track_branches_2 (Variables|TrackSetup|GetTrack%20Branches))
  (bind _output (Utilities|Array|Get(acopy) _track_branches_2))
  (LocalVariables|SetInserted%20Index Index)
  (for (_ _array_index) _track_branches
    (if (>= (.startingsplinepoint (Utilities|Array|Get(acopy) _track_branches _array_index)) (LocalVariables|GetInserted%20Index))
      (Utilities|Array|SetArrayElem _track_branches_2 _array_index (Utilities|Struct|MakeTrackBranchData (.branchactive (Utilities|Array|Get(acopy) _track_branches _array_index)) (+ (.startingsplinepoint (Utilities|Array|Get(acopy) _track_branches _array_index)) 1) (.endingsplinepoint (Utilities|Array|Get(acopy) _track_branches _array_index)) (.removebranch (Utilities|Array|Get(acopy) _track_branches _array_index)))))
    (if (>= (.endingsplinepoint _output) (LocalVariables|GetInserted%20Index))
      (Utilities|Array|SetArrayElem (Variables|TrackSetup|GetTrack%20Branches) _array_index (Utilities|Struct|MakeTrackBranchData (.branchactive _output) (.startingsplinepoint _output) (+ (.endingsplinepoint _output) 1) (.removebranch _output))))))

(fn NewFunction1
  (params (NewParam :type Array%20of%20Vectors) (NewParam1 :type Array%20of%20Vectors) (NewParam4 :type Integer))
  (bind _returnvalue (* NewParam4 2))
  (bind _output (Utilities|Array|Get(acopy) NewParam1 NewParam4))
  (bind _returnvalue_2 (+ _returnvalue 1))
  (bind _output_2 (Utilities|Array|Get(acopy) NewParam _returnvalue))
  (bind _output_3 (Utilities|Array|Get(acopy) NewParam _returnvalue_2))
  (bind _returnvalue_3 (- _output_3 _output))
  (bind _returnvalue_4 (- _output_3 _output_2))
  (bind _returnvalue_5 (Math|Vector|Normalize _returnvalue_4 0.0))
  (return (* _returnvalue_5 (Class|KismetMathLibrary|VSizeXYSquared (- _output _output_2))) (Math|Vector|SelectVector (* _returnvalue_5 (Class|KismetMathLibrary|VSizeXYSquared _returnvalue_3)) _returnvalue_3 (== 0 NewParam4))))