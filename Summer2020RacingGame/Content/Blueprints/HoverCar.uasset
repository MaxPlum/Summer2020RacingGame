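; Player-driven physics hover car with throttle, strafing, jumping, ground turning, air rolling and a stick-angle camera, moved by forces and torques on CarMesh.
; Four hover components share gravity, while sensor components supply weighted floor normals averaged each tick into directional gravity, defaulting to world up.
; Tick also applies ground or air momentum.
; When reorientation checks flag the car upside down past a delay, it locks input, launches and rolls until CanJump returns.
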(event OnComponentSleep(HUD_time)
  (params (SleepingComponent :type Primitive%20Component%20Object%20Reference) (BoneName :type Name :default "None")))

(event OnComponentSleep(HUD_lap)
  (params (SleepingComponent :type Primitive%20Component%20Object%20Reference) (BoneName :type Name :default "None")))

(event OnComponentSleep(HUD_map)
  (params (SleepingComponent :type Primitive%20Component%20Object%20Reference) (BoneName :type Name :default "None")))

(event OnComponentSleep(HUD_revs)
  (params (SleepingComponent :type Primitive%20Component%20Object%20Reference) (BoneName :type Name :default "None")))

(event OnComponentSleep(HUD_sides)
  (params (SleepingComponent :type Primitive%20Component%20Object%20Reference) (BoneName :type Name :default "None")))

(event EventBeginPlay
  (bind _carmesh (Variables|Default|GetCarMesh))
  (bind _sensor_component_array (Variables|HoverCarComponents|GetSensor%20Component%20Array))
  (bind _sensorcomponentcenter (Variables|Default|GetSensorComponentCenter))
  (bind _reorientatecomponent (Variables|Default|GetReorientateComponent))
  ;[1 1 1] HOVER CAR COMPONENTS (Initialize Components)
  (bind _returnvalue (UserInterface|CreateWidget "/Game/Blueprints/HUD_Widget.HUD_Widget_C" (Game|GetPlayerController 0)))
  (UserInterface|Viewport|AddtoViewport _returnvalue 0)
  ;;[1 1 1] Saves Parent ID For Hover Component
  (bind _outactors (Actor|GetAllActorsOfClass "HoverCar_C"))
  (bind (_array_element _array_index) (Utilities|Array|ForEachLoopwithBreak _outactors :!label _label)
    (:LoopBody
      (if (== _array_element self)
        (bind _output_get (Variables|HoverCarComponents|SetParent%20Index _array_index))
        (goto _label Break)))
    (:Completed
      (Default|InitializeHoverComponent (Variables|Default|GetHoverComponentFrontRight) _carmesh _output_get (/ (Variables|DirectionalGravity|GetGravity) 4.0))
      (Default|InitializeReorientateComponent _reorientatecomponent _carmesh)
      (Utilities|Array|AddUnique (Variables|HoverCarComponents|GetReorientation%20Component%20Array) _reorientatecomponent)
      (Default|InitializeSensorComponent _sensorcomponentcenter _carmesh)
      (Utilities|Array|AddUnique _sensor_component_array _sensorcomponentcenter)
      (Utilities|Array|AddUnique _sensor_component_array (Variables|Default|GetSensorComponentFrontRight))
      (Utilities|Array|AddUnique _sensor_component_array (Variables|Default|GetSensorComponentFrontLeft))
      (Utilities|Array|AddUnique _sensor_component_array (Variables|Default|GetSensorComponentBackLeft))
      (Utilities|Array|AddUnique _sensor_component_array (Variables|Default|GetSensorComponentBackRight)))))

(event EventTick
  (params (DeltaSeconds :type Float%20%28single-precision%29))
  (bind _carmesh (Variables|Default|GetCarMesh))
  (bind _returnvalue (Transformation|GetComponentVelocity _carmesh))
  (CallFunction|GetSpeed)
  ;[1 1 1] MOMENTUM (Set Rolling Delay Timer & Clean Jump Requirement Each Update)
  (Variables|Turning/Rolling|SetRolling%20Delay%20Timer (- (Variables|Turning/Rolling|GetRolling%20Delay%20Timer) DeltaSeconds))
  (if (Variables|Jumping|GetJump%20Check)
    (Physics|AddForce _carmesh (* _returnvalue (Variables|Momentum|GetMomentum)) "None" false)
    (Variables|Turning/Rolling|SetRolling%20Delay%20Timer (Variables|Turning/Rolling|GetRolling%20Delay))
    (Variables|Jumping|SetJump%20Check false)
    (else
      (Physics|AddForce _carmesh (* _returnvalue (Variables|Momentum|GetIn%20Air%20Momentum)) "None" false)
      (Variables|Jumping|SetCan%20Jump false)))
  ;[1 1 1] DIRECTIONAL GRAVITY
  (Variables|DirectionalGravity|SetSensor%20Hits 0.0)
  (Variables|DirectionalGravity|SetGravity%20Vector "0, 0, 0")
  (for _array_element (Variables|HoverCarComponents|GetSensor%20Component%20Array)
    (CallFunction|CalculateGravityVector _array_element))
  (if (== (Variables|DirectionalGravity|GetSensor%20Hits) 0.0)
    (Variables|DirectionalGravity|SetGravity%20Vector "0, 0,1.000000")
    (else
      (Variables|DirectionalGravity|SetGravity%20Vector (/ (Variables|DirectionalGravity|GetGravity%20Vector) (Variables|DirectionalGravity|GetSensor%20Hits)))))
  (Physics|AddForce (Variables|Default|GetCarMesh) (* (Variables|DirectionalGravity|GetGravity%20Vector) (* -1 (Variables|DirectionalGravity|GetGravity))) "None" false)
  ;[1 1 1] REORIENTATION
  (if (Variables|Reorientation|GetInput%20Lock)
    (if (Variables|Jumping|GetCan%20Jump)
      (Variables|Reorientation|SetInput%20Lock false)
      (else
        (Class|PrimitiveComponent|AddTorqueinRadians (Variables|Default|GetCarMesh) (* (* (Math|Vector|GetForwardVector (Variables|Default|GetCarMesh)) -1) (Variables|Reorientation|GetReorientation%20Rolling%20Velocity)) "None" false)))
    (elif (not (Variables|Jumping|GetCan%20Jump))
      (Variables|Reorientation|SetUpside%20Down false)
      (for _array_element_2 (Variables|HoverCarComponents|GetReorientation%20Component%20Array)
        (bind _surface_hit (Default|GetReorientateCheck _array_element_2))
        (if _surface_hit
          (Variables|Reorientation|SetUpside%20Down true)))
      (if (Variables|Reorientation|GetUpside%20Down)
        (bind _output_get (Variables|Reorientation|SetReorientation%20Timer (- (Variables|Reorientation|GetReorientation%20Timer) (Utilities|Time|GetWorldDeltaSeconds))))
        (if (<= _output_get 0.0)
          (Variables|Reorientation|SetInput%20Lock true)
          (Physics|AddForce (Variables|Default|GetCarMesh) (* (Variables|DirectionalGravity|GetGravity%20Vector) (* (Variables|Reorientation|GetReorientation%20Launch%20Force) -1.0)) "None" false))
        (else
          (Variables|Reorientation|SetReorientation%20Timer (Variables|Reorientation|GetReorientation%20Delay)))))))

(event Input|ActionEvents|InputActionJump
  (params (Key :type Key%20Structure))
  ;[1 1 1] JUMPING
  (:Pressed
    (if (not (Variables|Reorientation|GetInput%20Lock))
      (if (Variables|Jumping|GetCan%20Jump)
        (Physics|AddForce (Variables|Default|GetCarMesh) (* (Variables|DirectionalGravity|GetGravity%20Vector) (Variables|Jumping|GetJump%20Force)) "None" false)
        (Variables|Jumping|SetCan%20Jump false)))))

(event Input|AxisEvents|InputAxisMoveRight
  (params (AxisValue :type Float%20%28single-precision%29))
  (bind _carmesh (Variables|Default|GetCarMesh))
  (bind _carmesh_2 (Variables|Default|GetCarMesh))
  ;[1 1 1] TURNING/ROLLING
  (if (not (Variables|Reorientation|GetInput%20Lock))
    (bind _returnvalue (Physics|GetPhysicsLinearVelocity _carmesh "None"))
    ;;[1 1 1] Determine Whether To Turn Or Roll And Set Variables Accordingly. If Rolling, Check Delay Timer
    (if (Variables|Jumping|GetJump%20Check)
      (Variables|Turning/Rolling|SetRotation%20Direction%20Vector (Math|Vector|GetUpVector _carmesh_2))
      (Variables|Turning/Rolling|SetRotation%20Velocity (Variables|Turning/Rolling|GetTurning%20Velocity))
      (Class|PrimitiveComponent|AddTorqueinRadians (Variables|Default|GetCarMesh) (* (Variables|Turning/Rolling|GetRotation%20Direction%20Vector) (* (Math|Float|SelectFloat -1.0 1.0 (<= (Math|Conversions|ToFloat(Integer) (Math|Float|Truncate (Math|Vector|DotProduct _returnvalue (Math|Vector|GetForwardVector _carmesh)))) -1e+02)) (* AxisValue (Variables|Turning/Rolling|GetRotation%20Velocity)))) "None" false :!label _label)
      (elif (<= (Variables|Turning/Rolling|GetRolling%20Delay%20Timer) 0.0)
        (Variables|Turning/Rolling|SetRolling%20Delay%20Timer 0.0)
        (Variables|Turning/Rolling|SetRotation%20Direction%20Vector (* (Math|Vector|GetForwardVector _carmesh_2) -1))
        (Variables|Turning/Rolling|SetRotation%20Velocity (Variables|Turning/Rolling|GetRolling%20Velocity))
        (goto _label)))))

(event Input|AxisEvents|InputAxisStrafeLeft
  (params (AxisValue :type Float%20%28single-precision%29))
  ;[1 1 1] STRAFING
  (if (not (Variables|Reorientation|GetInput%20Lock))
    (Physics|AddForce (Variables|Default|GetCarMesh) (* (* (Math|Vector|GetRightVector (Variables|Default|GetCarMesh)) (+ (stale Input|AxisEvents|InputAxisStrafeRight AxisValue) (* -1 AxisValue))) (Variables|Strafing|GetStrafe%20Speed)) "None" false)))

(event Input|AxisEvents|InputAxisStrafeRight
  (params (AxisValue :type Float%20%28single-precision%29))
  ;[1 1 1] STRAFING
  (if (not (Variables|Reorientation|GetInput%20Lock))
    (Physics|AddForce (Variables|Default|GetCarMesh) (* (* (Math|Vector|GetRightVector (Variables|Default|GetCarMesh)) (+ AxisValue (* -1 (stale Input|AxisEvents|InputAxisStrafeLeft AxisValue)))) (Variables|Strafing|GetStrafe%20Speed)) "None" false)))

(event Input|AxisEvents|InputAxisMoveForward
  (params (AxisValue :type Float%20%28single-precision%29))
  (bind _carmesh (Variables|Default|GetCarMesh))
  ;[1 1 1] FORWARD/BACKWARD MOVEMENT
  (if (not (Variables|Reorientation|GetInput%20Lock))
    (if (Variables|Jumping|GetJump%20Check)
      (Physics|AddForce (Variables|Default|GetCarMesh) (* (* (* (Math|Vector|GetForwardVector (Variables|Default|GetCarMesh)) (* (Variables|Forward/BackwardMovement|GetAcceleration) (+ (/ (Math|Vector|VectorLength (* (Transformation|GetComponentVelocity _carmesh) (Math|Vector|GetForwardVector _carmesh))) 1.5e+04) 0.1))) (+ AxisValue (stale Input|AxisEvents|InputAxisMoveBackwards AxisValue))) (Math|Float|SelectFloat (Variables|Forward/BackwardMovement|GetForward%20Acceleration%20Percentage) (Variables|Forward/BackwardMovement|GetReverse%20Acceleration%20Percentage) (>= (+ AxisValue (stale Input|AxisEvents|InputAxisMoveBackwards AxisValue)) 0.0))) "None" false)
      (else
        (Physics|AddForce (Variables|Default|GetCarMesh) (* (Transformation|GetComponentVelocity (Variables|Default|GetCarMesh)) 0.2) "None" false)))))

(event Input|AxisEvents|InputAxisMoveBackwards
  (params (AxisValue :type Float%20%28single-precision%29))
  (bind _carmesh (Variables|Default|GetCarMesh))
  ;[1 1 1] FORWARD/BACKWARD MOVEMENT
  (if (not (Variables|Reorientation|GetInput%20Lock))
    (if (Variables|Jumping|GetJump%20Check)
      (Physics|AddForce (Variables|Default|GetCarMesh) (* (* (* (Math|Vector|GetForwardVector (Variables|Default|GetCarMesh)) (* (Variables|Forward/BackwardMovement|GetAcceleration) (+ (/ (Math|Vector|VectorLength (* (Transformation|GetComponentVelocity _carmesh) (Math|Vector|GetForwardVector _carmesh))) 1.5e+04) 0.1))) (+ (stale Input|AxisEvents|InputAxisMoveForward AxisValue) AxisValue)) (Math|Float|SelectFloat (Variables|Forward/BackwardMovement|GetForward%20Acceleration%20Percentage) (Variables|Forward/BackwardMovement|GetReverse%20Acceleration%20Percentage) (>= (+ (stale Input|AxisEvents|InputAxisMoveForward AxisValue) AxisValue) 0.0))) "None" false)
      (else
        (Physics|AddForce (Variables|Default|GetCarMesh) (* (Transformation|GetComponentVelocity (Variables|Default|GetCarMesh)) 0.2) "None" false)))))

(event Input|AxisEvents|InputAxisTurnRate
  (params (AxisValue :type Float%20%28single-precision%29))
  ;[1 1 1] Camera Rotation
  (CallFunction|RotateCamera AxisValue (stale Input|AxisEvents|InputAxisLookUpRate AxisValue)))

(event Input|AxisEvents|InputAxisLookUpRate
  (params (AxisValue :type Float%20%28single-precision%29))
  ;[1 1 1] Camera Rotation
  (CallFunction|RotateCamera (stale Input|AxisEvents|InputAxisTurnRate AxisValue) AxisValue))

(fn ConstructionScript)

(fn CalculateGravityVector
  (params (Sensor%20Component :type Sensor%20Component%20Object%20Reference))
  (bind (_surface_hit _floor_normal _hit_weight) (Default|GetFloorNormal Sensor%20Component))
  (if _surface_hit
    (Variables|DirectionalGravity|SetGravity%20Vector (+ (* _floor_normal _hit_weight) (Variables|DirectionalGravity|GetGravity%20Vector)))
    (Variables|DirectionalGravity|SetSensor%20Hits (+ _hit_weight (Variables|DirectionalGravity|GetSensor%20Hits)))))

(fn RotateCamera
  (params (Horizontal%20Axis :type Float%20%28single-precision%29) (Vertical%20Axis :type Float%20%28single-precision%29))
  (LocalVariables|SetX%20Axis Horizontal%20Axis)
  (LocalVariables|SetY%20Axis Vertical%20Axis)
  (if (and (or (== (LocalVariables|GetX%20Axis) 1.0) (== (LocalVariables|GetX%20Axis) -1.0)) (== (LocalVariables|GetY%20Axis) 0.0))
    (if (== (LocalVariables|GetX%20Axis) 1.0)
      (LocalVariables|SetCamera%20Angle 2.7e+02)
      (else
        (LocalVariables|SetCamera%20Angle 9e+01)))
    (elif (>= (LocalVariables|GetY%20Axis) 0.0)
      (LocalVariables|SetCamera%20Angle (* (Class|KismetMathLibrary|DegAtan (/ (LocalVariables|GetX%20Axis) (LocalVariables|GetY%20Axis))) -1.0))
      (else
        (LocalVariables|SetCamera%20Angle (- 1.8e+02 (Class|KismetMathLibrary|DegAtan (/ (LocalVariables|GetX%20Axis) (LocalVariables|GetY%20Axis))))))))
  (Transformation|SetRelativeRotation (Variables|Default|GetSpringArm) (Math|Rotator|MakeRotator 0.0 0.0 (LocalVariables|GetCamera%20Angle)) false false))

(fn GetSpeed
  (bind _carmesh (Variables|Default|GetCarMesh))
  (Variables|Default|SetSpeed (Math|Float|Clamp(Float) (/ (Math|Vector|VectorLength (* (Transformation|GetComponentVelocity _carmesh) (Math|Vector|GetForwardVector _carmesh))) 1.5e+04))))