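; Modular building actor with optional awning, front and side rails, roof, and one of five vent positions.
; The construction script turns the vent enum into exclusive toggles, sets each detail mesh's visibility, and assigns the building mesh's material from a color enum.
; BeginPlay disables collision on every detail that is toggled off, since the construction script only handles visibility and material.
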(event EventBeginPlay
  ;[1 1 1] Set Collision To None If Detail Is Not Visible
  (CallFunction|UpdateCollision (Variables|Default|GetAwning%20Mesh) (Variables|Visibility|GetToggle%20Awning))
  (CallFunction|UpdateCollision (Variables|Default|GetFront%20Rail%20Mesh) (Variables|Visibility|GetToggle%20Rails%20-%20Front))
  (CallFunction|UpdateCollision (Variables|Default|GetSide%20Rail%20Mesh) (Variables|Visibility|GetToggle%20Rails%20-%20Side))
  (CallFunction|UpdateCollision (Variables|Default|GetRoof%20Mesh) (Variables|Visibility|GetToggle%20Roof))
  (CallFunction|UpdateCollision (Variables|Default|GetVent%201%20Mesh) (Variables|Visibility|GetToggle%20Vent%20-%201))
  (CallFunction|UpdateCollision (Variables|Default|GetVent%202%20Mesh) (Variables|Visibility|GetToggle%20Vent%20-%202))
  (CallFunction|UpdateCollision (Variables|Default|GetVent%203%20Mesh) (Variables|Visibility|GetToggle%20Vent%20-%203))
  (CallFunction|UpdateCollision (Variables|Default|GetVent%204%20Mesh) (Variables|Visibility|GetToggle%20Vent%20-%204))
  (CallFunction|UpdateCollision (Variables|Default|GetVent%205%20Mesh) (Variables|Visibility|GetToggle%20Vent%20-%205)))

(event Collision|EventActorBeginOverlap
  (params (OtherActor :type Actor%20Object%20Reference)))

(event EventTick
  (params (DeltaSeconds :type Float%20%28single-precision%29)))

(fn ConstructionScript
  ;[1 1 1] Toggle Component Visibility And Collision
  (CallFunction|HandleVentSelection)
  (Rendering|SetVisibility (Variables|Default|GetAwning%20Mesh) (Variables|Visibility|GetToggle%20Awning) false)
  (Rendering|SetVisibility (Variables|Default|GetFront%20Rail%20Mesh) (Variables|Visibility|GetToggle%20Rails%20-%20Front) false)
  (Rendering|SetVisibility (Variables|Default|GetSide%20Rail%20Mesh) (Variables|Visibility|GetToggle%20Rails%20-%20Side) false)
  (Rendering|SetVisibility (Variables|Default|GetRoof%20Mesh) (Variables|Visibility|GetToggle%20Roof) false)
  (Rendering|SetVisibility (Variables|Default|GetVent%201%20Mesh) (Variables|Visibility|GetToggle%20Vent%20-%201) false)
  (Rendering|SetVisibility (Variables|Default|GetVent%202%20Mesh) (Variables|Visibility|GetToggle%20Vent%20-%202) false)
  (Rendering|SetVisibility (Variables|Default|GetVent%203%20Mesh) (Variables|Visibility|GetToggle%20Vent%20-%203) false)
  (Rendering|SetVisibility (Variables|Default|GetVent%204%20Mesh) (Variables|Visibility|GetToggle%20Vent%20-%204) false)
  (Rendering|SetVisibility (Variables|Default|GetVent%205%20Mesh) (Variables|Visibility|GetToggle%20Vent%20-%205) false)
  ;[1 1 1] Set Object Texture
  (CallFunction|UpdateTexture-BuildingUnit (Variables|Default|GetBuilding%20Mesh) (Variables|Texture|GetBuilding%20Texture)))

(fn UpdateCollision
  (params (Mesh :type Static%20Mesh%20Component%20Object%20Reference) (Toggle :type Boolean))
  (if (not Toggle)
    (Collision|SetCollisionEnabled Mesh "NoCollision")))

(fn UpdateTexture-BuildingUnit
  (params (Mesh :type Static%20Mesh%20Component%20Object%20Reference) (Texture%20Enum :type Texture_Enum-Building_Unit%20Enum :default "NewEnumerator0"))
  (switch Utilities|FlowControl|Switch|SwitchonTexture_Enum-Building_Unit Texture%20Enum
    (:NewEnumerator0
      (Rendering|Material|SetMaterial Mesh 0 "/Game/Architecture/Buildings/Materials/M_Building_Master_Inst.M_Building_Master_Inst"))
    (:NewEnumerator1
      (Rendering|Material|SetMaterial Mesh 0 "/Game/Architecture/Buildings/Materials/M_Awning_Master_Inst.M_Awning_Master_Inst"))
    (:NewEnumerator2
      (Rendering|Material|SetMaterial Mesh 0 "/Game/Architecture/Buildings/Materials/M_Rails_Master_Inst.M_Rails_Master_Inst"))))

(fn HandleVentSelection
  (Variables|Visibility|SetToggle%20Vent%20-%201 false)
  (Variables|Visibility|SetToggle%20Vent%20-%202 false)
  (Variables|Visibility|SetToggle%20Vent%20-%203 false)
  (Variables|Visibility|SetToggle%20Vent%20-%204 false)
  (Variables|Visibility|SetToggle%20Vent%20-%205 false)
  (switch Utilities|FlowControl|Switch|SwitchonBuilding_Unit_Enum-Select_Vent (Variables|Visibility|GetVent%20Selection)
    (:NewEnumerator0
      (Variables|Visibility|SetToggle%20Vent%20-%201 true))
    (:NewEnumerator1
      (Variables|Visibility|SetToggle%20Vent%20-%202 true))
    (:NewEnumerator2
      (Variables|Visibility|SetToggle%20Vent%20-%203 true))
    (:NewEnumerator3
      (Variables|Visibility|SetToggle%20Vent%20-%204 true))
    (:NewEnumerator4
      (Variables|Visibility|SetToggle%20Vent%20-%205 true))))