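; Sensor component that detects the surface beneath it and records that surface's normal.
; Each tick it line traces on the Visibility channel along its own negative up vector for TraceLength, with per-frame debug drawing.
; GetFloorNormal returns the hit flag and the impact normal, which keeps its last value when the trace misses.
; An initialize event stores a parent mesh reference, which this graph does not otherwise use.
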(event Custom|Initialize%20Sensor%20Component
  (params (Mesh%20Component :type Static%20Mesh%20Component%20Object%20Reference))
  ;[1 1 1] Initialize Sensor Component
  (Variables|Default|SetParent%20Component Mesh%20Component))

(event EventTick
  (params (DeltaSeconds :type Float%20%28single-precision%29))
  (bind _returnvalue (Transformation|GetWorldLocation))
  (Variables|Default|SetSurface%20Hit false)
  (bind (_outhit _returnvalue_2) (Collision|LineTraceByChannel _returnvalue (+ _returnvalue (* (Math|Vector|GetUpVector) (* (Variables|Default|GetTrace%20Length) -1.0))) "TraceTypeQuery1" false 0 "ForOneFrame" true "(R=0.046698,G=0.000000,B=1.000000,A=1.000000)"))
  (if _returnvalue_2
    (Variables|Default|SetSurface%20Hit true)
    (Variables|Default|SetFloor%20Angle (.ImpactNormal (Collision|BreakHitResult _outhit)))))

(fn GetFloorNormal
  (return (Variables|Default|GetSurface%20Hit) (Variables|Default|GetFloor%20Angle)))