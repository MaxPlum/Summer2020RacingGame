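; Hover component that pushes a physics-simulated mesh away from the surface beneath it.
; Initialization stores the given mesh as the parent and enables physics simulation on it.
; Each tick, a debug-drawn Visibility trace runs along the component's local down axis.
; On a hit, it applies force along the impact normal at its own location, fading linearly with distance, and sets the mesh's linear and angular damping.
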(event Custom|Initialize%20Hover%20Component
  (params (Mesh%20Component :type Static%20Mesh%20Component%20Object%20Reference))
  ;[1 1 1] Initialize Hover Component
  (bind _output_get (Variables|Default|SetParent%20Component Mesh%20Component))
  (Physics|SetSimulatePhysics _output_get true))

(event EventTick
  (params (DeltaSeconds :type Float%20%28single-precision%29))
  (bind _returnvalue (Transformation|GetWorldLocation))
  (bind (_outhit _returnvalue_2) (Collision|LineTraceByChannel _returnvalue (+ _returnvalue (* (Math|Vector|GetUpVector) (* (Variables|Default|GetTrace%20Length) -1.0))) "TraceTypeQuery1" false 0 "ForOneFrame"))
  (if _returnvalue_2
    (Class|PrimitiveComponent|AddForceatLocation (Variables|Default|GetParent%20Component) (* (.ImpactNormal (Collision|BreakHitResult _outhit)) (Math|Float|Lerp (Variables|Default|GetHover%20Force) 0.0 (/ (Math|Vector|VectorLength (- (.Location (Collision|BreakHitResult _outhit)) (Transformation|GetWorldLocation))) (Variables|Default|GetTrace%20Length)))) (Transformation|GetWorldLocation) "None")
    (Class|PrimitiveComponent|SetLinearDamping (Variables|Default|GetParent%20Component) (Variables|Default|GetLinear%20Damping))
    (Class|PrimitiveComponent|SetAngularDamping (Variables|Default|GetParent%20Component) (Variables|Default|GetAngular%20Damping))))